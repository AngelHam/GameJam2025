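; Player stats component that tracks health and stamina, plus a separate enemy health value, with current and max amounts.
; BeginPlay caches the player's BP_MyCharacter, whose HUDWidget bars and text every change function updates directly.
; Increases clamp to the max, decreases floor at zero and return true on depletion.
; Max health and stamina can be raised, and one helper raises current and max health together.
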(event `self.ReceiveBeginPlay`
  (bind _asbp_my_character (cast `/Game/GameJam/BP_MyCharacter` (`GameplayStatics.GetPlayerCharacter` 0)))
  (set `self.Player character BP` _asbp_my_character))

(fn `Decrease Health`
  (params (Damage :type "Float (double-precision)"))
  (returns (`Is Player Dead` :type Boolean))
  (bind _hud_widget (`/Game/GameJam/BP_MyCharacter.HUD Widget` (`self.Player character BP`)))
  (bind _output_get (set `self.Current Health` (- (`self.Current Health`) Damage)))
  (`ProgressBar.SetPercent` (`/Game/GameJam/WB_HUD.HealthBar` _hud_widget) (/ _output_get (`self.Max Health`)))
  (if (<= (`self.Current Health`) 0.0)
    (set `self.Current Health` 0.0))
  (`TextBlock.SetText` (`/Game/GameJam/WB_HUD.HealthText` _hud_widget) (`KismetTextLibrary.Conv_DoubleToText` (`self.Current Health`) "HalfToEven"))
  (if (<= (`self.Current Health`) 0.0)
    (return true)
    (else
      (return false))))

(fn `Decrease Health_Enemy`
  (params (Damage :type "Float (double-precision)"))
  (returns (`Is Enemy Dead` :type Boolean))
  (bind _hud_widget (`/Game/GameJam/BP_MyCharacter.HUD Widget` (`self.Player character BP`)))
  (bind _output_get (set `self.Current Health_Enemy` (- (`self.Current Health_Enemy`) Damage)))
  (`ProgressBar.SetPercent` (`/Game/GameJam/WB_HUD.EnemyHealthBar` _hud_widget) (/ _output_get (`self.Max Health_Enemy`)))
  (if (<= (`self.Current Health_Enemy`) 0.0)
    (set `self.Current Health_Enemy` 0.0))
  (`TextBlock.SetText` (`/Game/GameJam/WB_HUD.EnemyHealthText` _hud_widget) (`KismetTextLibrary.Conv_DoubleToText` (`self.Current Health_Enemy`) "HalfToEven"))
  (if (<= (`self.Current Health_Enemy`) 0.0)
    (return true)
    (else
      (return false))))

(fn `Decrease Stamina`
  (params (`Stamina Decrement` :type "Float (double-precision)"))
  (returns (`No Stamina Left` :type Boolean))
  (bind _hud_widget (`/Game/GameJam/BP_MyCharacter.HUD Widget` (`self.Player character BP`)))
  (set `self.Current Stamina` (- (`self.Current Stamina`) `Stamina Decrement`))
  (`ProgressBar.SetPercent` (`/Game/GameJam/WB_HUD.StaminaBar` _hud_widget) (/ (`self.Current Stamina`) (`self.Max Stamina`)))
  (if (<= (`self.Current Stamina`) 0.0)
    (set `self.Current Stamina` 0.0))
  (`TextBlock.SetText` (`/Game/GameJam/WB_HUD.StaminaText` _hud_widget) (`KismetTextLibrary.Conv_DoubleToText` (`self.Current Stamina`) "HalfToEven"))
  (if (<= (`self.Current Stamina`) 0.0)
    (return true)
    (else
      (return false))))

(fn `Increase Curr and Max Health`
  (params (`Health Increment` :type "Float (double-precision)"))
  (`self.Increase MaxHealth` `Health Increment`)
  (`self.Increase Health` `Health Increment`))

(fn `Increase Health`
  (params (`Health Increment` :type "Float (double-precision)"))
  (bind _returnvalue (+ `Health Increment` (`self.Current Health`)))
  (bind _hud_widget (`/Game/GameJam/BP_MyCharacter.HUD Widget` (`self.Player character BP`)))
  (if (> _returnvalue (`self.Max Health`))
    (set `self.Current Health` (`self.Max Health`))
    (else
      (set `self.Current Health` _returnvalue)))
  (`ProgressBar.SetPercent` (`/Game/GameJam/WB_HUD.HealthBar` _hud_widget) (/ (`self.Current Health`) (`self.Max Health`)))
  (`TextBlock.SetText` (`/Game/GameJam/WB_HUD.HealthText` _hud_widget) (`KismetTextLibrary.Conv_DoubleToText` (`self.Current Health`) "HalfToEven")))

(fn `Increase Health_Enemy`
  (params (`Health Increment` :type "Float (double-precision)"))
  (bind _returnvalue (+ `Health Increment` (`self.Current Health_Enemy`)))
  (bind _hud_widget (`/Game/GameJam/BP_MyCharacter.HUD Widget` (`self.Player character BP`)))
  (if (> _returnvalue (`self.Max Health_Enemy`))
    (set `self.Current Health_Enemy` (`self.Max Health_Enemy`))
    (else
      (set `self.Current Health_Enemy` _returnvalue)))
  (`ProgressBar.SetPercent` (`/Game/GameJam/WB_HUD.EnemyHealthBar` _hud_widget) (/ (`self.Current Health_Enemy`) (`self.Max Health_Enemy`)))
  (`TextBlock.SetText` (`/Game/GameJam/WB_HUD.EnemyHealthText` _hud_widget) (`KismetTextLibrary.Conv_DoubleToText` (`self.Current Health_Enemy`) "HalfToEven")))

(fn `Increase MaxHealth`
  (params (`Max Health Incremention` :type "Float (double-precision)"))
  (bind _hud_widget (`/Game/GameJam/BP_MyCharacter.HUD Widget` (`self.Player character BP`)))
  (bind _output_get (set `self.Max Health` (+ `Max Health Incremention` (`self.Max Health`))))
  (`ProgressBar.SetPercent` (`/Game/GameJam/WB_HUD.HealthBar` _hud_widget) (/ (`self.Current Health`) _output_get))
  (`TextBlock.SetText` (`/Game/GameJam/WB_HUD.HealthText` _hud_widget) (`KismetTextLibrary.Conv_DoubleToText` (`self.Current Health`) "HalfToEven")))

(fn `Increase MaxStamina`
  (params (`Max Stamina Increment` :type "Float (double-precision)"))
  (bind _hud_widget (`/Game/GameJam/BP_MyCharacter.HUD Widget` (`self.Player character BP`)))
  (set `self.Max Stamina` (+ `Max Stamina Increment` (`self.Max Stamina`)))
  (`ProgressBar.SetPercent` (`/Game/GameJam/WB_HUD.StaminaBar` _hud_widget) (/ (`self.Current Stamina`) (`self.Max Stamina`)))
  (`TextBlock.SetText` (`/Game/GameJam/WB_HUD.StaminaText` _hud_widget) (`KismetTextLibrary.Conv_DoubleToText` (`self.Current Stamina`) "HalfToEven")))

(fn `Increase Stamina`
  (params (`Stamina Increment` :type "Float (double-precision)"))
  (bind _returnvalue (+ `Stamina Increment` (`self.Current Stamina`)))
  (bind _hud_widget (`/Game/GameJam/BP_MyCharacter.HUD Widget` (`self.Player character BP`)))
  (if (> _returnvalue (`self.Max Stamina`))
    (set `self.Current Stamina` (`self.Max Stamina`))
    (else
      (set `self.Current Stamina` _returnvalue)))
  (`ProgressBar.SetPercent` (`/Game/GameJam/WB_HUD.StaminaBar` _hud_widget) (/ (`self.Current Stamina`) (`self.Max Stamina`)))
  (`TextBlock.SetText` (`/Game/GameJam/WB_HUD.StaminaText` _hud_widget) (`KismetTextLibrary.Conv_DoubleToText` (`self.Current Stamina`) "HalfToEven")))