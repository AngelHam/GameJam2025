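; Victory trophy actor that, when PlayTrophy is called, unhides and plays an end-of-game box-opening reveal.
; One timeline shakes the box, swings its four flaps open and lifts the trophy out; after a delay, confetti spawns and a second timeline floats and spins it.
; Meanwhile it flags game over, destroys a BP_Enemy, plays music, then toggles that off and opens the Arena level about ten seconds later.
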(event `self.ReceiveBeginPlay`)

(event `PlayTrophy`
  (bind _defaultsceneroot (`self.DefaultSceneRoot`))
  (bind (_relativelocation_x _relativelocation_y _relativelocation_z) (`KismetMathLibrary.BreakVector` (`SceneComponent.RelativeLocation` (`self.DefaultSceneRoot`))))
  (bind (_relativelocation_x_2 _relativelocation_y_2) (`KismetMathLibrary.BreakVector` (`SceneComponent.RelativeLocation` _defaultsceneroot)))
  (`SceneComponent.SetHiddenInGame` (`self.DefaultSceneRoot`) false true)
  (`|ExecutionSequence`
    (:`then_0`
      (bind (_direction _box_rotation _trophy_rotation _box_shake_location_z _box_shake_rotation_x _box_shake_rotation_y _boxshake_rot_z) (`Timeline|Timeline`)
        (:`Update`
          (`|ExecutionSequence`
            (:`then_0`
              (`SceneComponent.K2_SetRelativeLocationAndRotation` _defaultsceneroot (`KismetMathLibrary.MakeVector` _relativelocation_x_2 _relativelocation_y_2 (`KismetMathLibrary.Lerp` 0.0 100.0 _box_shake_location_z)) (`KismetMathLibrary.MakeRotator` (`KismetMathLibrary.Lerp` 0.0 25.0 _box_shake_rotation_x) (`KismetMathLibrary.Lerp` 0.0 20.0 _box_shake_rotation_y) (`KismetMathLibrary.Lerp` 0.0 10.0 _boxshake_rot_z)) false false))
            (:`then_1`
              (`SceneComponent.K2_SetRelativeRotation` (`self.sm_box_flapA`) (`KismetMathLibrary.MakeRotator` (`KismetMathLibrary.Lerp` 0.0 -147.0 _box_rotation)) false false)
              (`SceneComponent.K2_SetRelativeRotation` (`self.sm_box_flapA1`) (`KismetMathLibrary.MakeRotator` (`KismetMathLibrary.Lerp` 0.0 -118.0 _box_rotation) 0.0 -180.0) false false)
              (`SceneComponent.K2_SetRelativeRotation` (`self.sm_box_flapB`) (`KismetMathLibrary.MakeRotator` 0.0 (`KismetMathLibrary.Lerp` 0.0 -165.0 _box_rotation)) false false)
              (`SceneComponent.K2_SetRelativeRotation` (`self.sm_box_flapB1`) (`KismetMathLibrary.MakeRotator` 0.0 (`KismetMathLibrary.Lerp` 0.0 -189.0 _box_rotation) -180.0) false false))
            (:`then_2`
              (`SceneComponent.K2_SetRelativeLocationAndRotation` (`self.sm_trophy`) (`KismetMathLibrary.VLerp` (38.0 20.0 14.0) (0.0 0.0 50.0) _trophy_rotation) (`KismetMathLibrary.RLerp` (struct :`Yaw` -70.0 :`Roll` -90.0) (struct) _trophy_rotation) false false))))))
    (:`then_1`
      (`KismetSystemLibrary.Delay` 2.5)
      (`NiagaraFunctionLibrary.SpawnSystemAtLocation` "/Game/ParticleSystems/P_trophyConfetti.P_trophyConfetti" (`KismetMathLibrary.MakeVector` _relativelocation_x _relativelocation_y (+ _relativelocation_z 25.0)))
      (bind (_direction_2 _trophyspin _trophy_float) (`Timeline|Timeline_0`)
        (:`Update`
          (`SceneComponent.K2_SetRelativeLocationAndRotation` (`self.Scene`) (`KismetMathLibrary.MakeVector` 0.0 0.0 (`KismetMathLibrary.Lerp` 0.0 40.0 _trophy_float)) (`KismetMathLibrary.MakeRotator` 0.0 0.0 (`KismetMathLibrary.Lerp` 0.0 360.0 _trophyspin)) false false))))
    (:`then_2`
      (set `self.isGameOver?` true)
      (bind _returnvalue (`GameplayStatics.GetActorOfClass` "/Game/GameJam/BP_Enemy.BP_Enemy_C"))
      (`self.K2_DestroyActor` _returnvalue)
      (bind _returnvalue_2 (`GameplayStatics.SpawnSound2D` "/Game/Music/Canal_3_-_Quincas_Moreira.Canal_3_-_Quincas_Moreira" 1.0 1.0 0.0 null))
      (`KismetSystemLibrary.Delay` 10.0)
      (`ActorComponent.ToggleActive` _returnvalue_2)
      ; end current level music
      (`KismetSystemLibrary.Delay` 0.1)
      (`GameplayStatics.OpenLevelBySoftObjectPtr` "/Game/Arena.Arena"))))

(fn `UserConstructionScript`)