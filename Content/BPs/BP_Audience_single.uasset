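; BP_Audience_single is one audience member, a billboard with a chair, that bobs in place to animate a crowd.
; Construction picks a random billboard material and chair mesh from arrays.
; On BeginPlay, a timeline starts at a random position and play rate to desynchronise instances, driving scaled vertical movement.
; Its roll output is immediately overwritten by a zero-rotation call, and a random X offset node is unconnected.
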(event `self.ReceiveBeginPlay`
  (bind _timeline (`self.Timeline`))
  (`TimelineComponent.SetPlaybackPosition` _timeline (`KismetMathLibrary.RandomFloatInRange` 0.0 1.0) false true)
  (`TimelineComponent.SetPlayRate` _timeline (`KismetMathLibrary.RandomFloatInRange` 0.75 1.5))
  (bind (_direction _x_rotation _z_position) (`Timeline|Timeline`)
    (:`Update`
      (`SceneComponent.K2_SetRelativeLocationAndRotation` (`self.Audience`) (`KismetMathLibrary.MakeVector` (`self.New Location X`) 0.0 (* _z_position (`self.Z Position Multiply`))) (`KismetMathLibrary.MakeRotator` _x_rotation) false false)
      (`SceneComponent.K2_SetRelativeRotation` (`self.Audience`) (`KismetMathLibrary.MakeRotator` 0.0) false false))))

(fn `UserConstructionScript`
  (bind _chairmesharray (`self.chairMeshArray`))
  (bind _materialarray (`self.materialArray`))
  (`PrimitiveComponent.SetMaterial` (`self.audienceBillboard`) 0 (`|GetArrayItem` _materialarray (- (`KismetMathLibrary.RandomIntegerInRange` 1 (`KismetArrayLibrary.Array_Length` _materialarray)) 1)))
  (`StaticMeshComponent.SetStaticMesh` (`self.sm_chair_01`) (`|GetArrayItem` _chairmesharray (- (`KismetMathLibrary.RandomIntegerInRange` 1 (`KismetArrayLibrary.Array_Length` _chairmesharray)) 1))))