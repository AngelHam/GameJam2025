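; BP_audience_group spawns a row of BP_Audience_single actors at BeginPlay to form a crowd.
; Each is offset along local Y by index times Spacing, with its Audience component randomly shifted in X and Z for variety.
; SeatCapacity is the chance a seat looks occupied; otherwise the member's billboard is hidden in game, though the actor still spawns.
; The construction script stretches Scene's Y scale by Amount / 0.933, as Spacing cancels out.
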(event `self.ReceiveBeginPlay`
  (bind _defaultsceneroot (`self.DefaultSceneRoot`))
  (for _index (range (`self.Amount`))
    (bind _returnvalue (`|SpawnActorFromClass` "/Game/BPs/BP_Audience_single.BP_Audience_single_C" (`KismetMathLibrary.MakeTransform` (`SceneComponent.K2_GetComponentLocation` _defaultsceneroot) (`SceneComponent.RelativeRotation` _defaultsceneroot)) "Undefined" "MultiplyWithRoot" null null))
    (`|ExecutionSequence`
      (:`then_0`
        (bind _output_get (set `/Game/BPs/BP_Audience_single.Z Position Multiply` (`KismetMathLibrary.RandomFloatInRange` 0.5 2.5) _returnvalue))
        (bind _output_get_2 (set `/Game/BPs/BP_Audience_single.New Location X` (`KismetMathLibrary.RandomFloatInRange` -17.0 17.0) _returnvalue))
        (`SceneComponent.K2_SetRelativeLocation` (`/Game/BPs/BP_Audience_single.Audience` _returnvalue) (`KismetMathLibrary.MakeVector` _output_get_2 0.0 _output_get) false false))
      (:`then_1`
        (`self.K2_AddActorLocalOffset` _returnvalue (`KismetMathLibrary.MakeVector` 0.0 (* _index (`self.Spacing`))) false false))
      (:`then_2`
        (if (not (`KismetMathLibrary.RandomBoolWithWeight` (`self.Seat Capacity`)))
          (`SceneComponent.SetHiddenInGame` (`/Game/BPs/BP_Audience_single.audienceBillboard` _returnvalue) true false))))))

(fn `UserConstructionScript`
  (bind _scene (`self.Scene`))
  (bind (_relativescale3d_x _relativescale3d_y _relativescale3d_z) (`KismetMathLibrary.BreakVector` (`SceneComponent.RelativeScale3D` _scene)))
  (`SceneComponent.SetRelativeScale3D` _scene (`KismetMathLibrary.MakeVector` _relativescale3d_x (* _relativescale3d_y (/ (`self.Spacing`) (* (/ (`self.Spacing`) (`self.Amount`)) 0.933))) _relativescale3d_z)))